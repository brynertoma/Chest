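; BP_Chest is a chest with an emissive tint whose lid opens and closes when ToggleOpen is called.
; A FlipFlop plays a timeline forward or in reverse, interpolating the rotation of the Top component.
; The construction script applies one dynamic material with configurable emissive color and strength to both halves.
; It also scales an optionally visible sphere from NetCullDistanceSquared to visualize the network relevancy area.
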(event `ToggleOpen`
  (`/Engine/EditorBlueprintResources/StandardMacros.FlipFlop`
    (:`A`
      (bind (_direction _alpha) (`Timeline|OpenChestTimeline` :!via `PlayFromStart` :!label _label)
        (:`Update`
          (`SceneComponent.K2_SetRelativeRotation` (`self.Top`) (`KismetMathLibrary.RLerp` (struct) (struct :`Pitch` 130.0) _alpha) false false))))
    (:`B`
      (goto _label :!via `ReverseFromEnd`))))

(fn `SetMaterial`
  (locals (Material :type "MaterialInstanceDynamic Object Reference"))
  (bind _returnvalue (`KismetMaterialLibrary.CreateDynamicMaterialInstance` null))
  (`PrimitiveComponent.SetMaterial` (`self.Top`) 0 _returnvalue)
  (`PrimitiveComponent.SetMaterial` (`self.Bottom`) 0 _returnvalue)
  (`MaterialInstanceDynamic.SetVectorParameterValue` _returnvalue "EmissiveColor" (`self.EmissiveColor`))
  (`MaterialInstanceDynamic.SetScalarParameterValue` _returnvalue "EmissiveStrength" (`self.EmissiveStrength`)))

(fn `UserConstructionScript`
  (`SceneComponent.SetWorldScale3D` (`self.Sphere`) (`KismetMathLibrary.Conv_DoubleToVector` (* 2 (`KismetMathLibrary.Sqrt` (`self.NetCullDistanceSquared`)))))
  (`SceneComponent.SetVisibility` (`self.Sphere`) (`self.ShowRelevancyArea?`) false)
  (`self.SetMaterial`))